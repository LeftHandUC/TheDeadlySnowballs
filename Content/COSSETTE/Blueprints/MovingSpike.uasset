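; MovingSpike is an enemy actor that moves along a timeline-driven path and can be destroyed by tapping or clicking it.
; On BeginPlay it stores its location, then a Timeline adds an offset to that origin on each update, setting the location without sweep.
; Touch and click on the static mesh share one path that decrements its life and destroys the actor at zero.
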(event OnInputTouchBegin(StaticMesh)
  (params (FingerIndex :type ETouchIndex%20Enum :default "Touch1") (TouchedComponent :type Primitive%20Component%20Object%20Reference))
  (Variables|Default|SetEnemy's%20Life (- (Variables|Default|GetEnemy's%20Life) 1))
  (if (<= (Variables|Default|GetEnemy's%20Life) 0)
    (Actor|DestroyActor)))

(event OnClicked(StaticMesh)
  (params (TouchedComponent :type Primitive%20Component%20Object%20Reference) (ButtonPressed :type Key%20Structure))
  (Variables|Default|SetEnemy's%20Life (- (Variables|Default|GetEnemy's%20Life) 1))
  (if (<= (Variables|Default|GetEnemy's%20Life) 0)
    (Actor|DestroyActor)))

(event EventBeginPlay
  (Variables|Default|SetInitial%20Variable (Transformation|GetActorLocation))
  (bind _enemy (Timeline|Timeline_0 PlayFromStart)
    (:Update
      (Transformation|SetActorLocation (+ (Variables|Default|GetInitial%20Variable) _enemy) false false))))

(fn ConstructionScript)